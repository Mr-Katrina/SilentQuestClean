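; Grey Child monster that roams at random and chases the player on sight, ending the run when it touches the VR pawn.
; Pawn sensing triggers an AI move toward the player, falling back to random reachable points on failure, with an attack montage gated by CanAttack.
; A capsule hit resets the first Grey Child found to roaming, then once disables player movement, plays a fade-out sequence and death sound, and loads the Cafe level.
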(event `self.ReceiveBeginPlay`
  (`self.Roaming`))

(event `self.PawnSensing.OnSeePawn`
  (params (Pawn :type "Pawn Object Reference"))
  (set `self.isSeeingPlayer?` true)
  (`self.FollowPlayer`))

(event `FollowPlayer`
  (set `self.canAttack` true)
  (if (`self.isSeeingPlayer?`)
    (`|AIMoveTo` self (0.0 0.0 0.0) (`GameplayStatics.GetPlayerCharacter` 0)
      (:`OnSuccess`
        (if (not (`self.canAttack`))
          (set `self.canAttack` false)
          (bind _returnvalue (`self.PlayAnimMontage` "/Game/Characters/Monsters/GreyCld/GreyChild_AttackMontage.GreyChild_AttackMontage"))
          (`KismetSystemLibrary.Delay` _returnvalue)
          (set `self.canAttack` true)))
      (:`OnFail`
        (`|AIMoveTo` self (`NavigationSystemV1.K2_GetRandomReachablePointInRadius` (`self.K2_GetActorLocation`) 1000.0 null null) null :!label _label
          (:`OnSuccess`
            (`self.Roaming`)))))
    (else
      (set `self.isSeeingPlayer?` false))))

(event `Roaming`
  (if (not (`self.isSeeingPlayer?`))
    (goto _label)))

(event `self.CapsuleComponent.OnComponentHit`
  (params (HitComponent :type "PrimitiveComponent Object Reference") (OtherActor :type "Actor Object Reference") (OtherComp :type "PrimitiveComponent Object Reference") (NormalImpulse :type "Vector Structure") (Hit :type "HitResult Structure (by ref)"))
  (cast `/Game/Player/VRPawn` OtherActor)
  (bind _outactors (`GameplayStatics.GetAllActorsOfClass` "BP_GreyChild_C"))
  (bind _output (`|GetArrayItem` _outactors))
  (`self.Roaming` _output)
  (set `/Game/Characters/Monsters/GreyCld/BP_GreyChild.canAttack` false _output)
  (`/Engine/EditorBlueprintResources/StandardMacros.DoOnce` false
    (:`Completed`
      (`/Game/VisualEffects/Font/2d_scenes/2d_scenes1/StoryAdvTemplate/Blueprints/Core/BP_StoryAdv_FunctionLibrary.DisablePlayerMovement`)
      (bind _outactors_2 (`GameplayStatics.GetAllActorsOfClass` "/Script/LevelSequence.LevelSequenceActor"))
      (`LevelSequenceActor.SetSequence` _outactors_2 (`self.FadeOut`))
      (`MovieSceneSequencePlayer.Play` (`LevelSequenceActor.SequencePlayer` (`|GetArrayItem` _outactors_2)))
      (`KismetSystemLibrary.Delay` 0.5)
      (`GameplayStatics.PlaySound2D` "/Game/Sound/SE/SE_HarryDie.SE_HarryDie" 1.0 1.0 0.0 null null)
      (`KismetSystemLibrary.Delay` 3.0)
      (`GameplayStatics.OpenLevel` "Cafe"))))

(fn `UserConstructionScript`)