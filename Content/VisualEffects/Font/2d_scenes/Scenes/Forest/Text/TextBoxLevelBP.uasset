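; Forest level dialogue actor that plays a three-message text box sequence when its level-start event fires, with player movement locked.
; Each message sets TextSetter and spawns a fresh Text_forestLevelBP widget, with a length-based delay marking when typing finishes.
; Interact zeroes the letter delay mid-typing or advances to the next message, with sound.
; After the last, it restores movement, calls CallFinishedTalking and destroys itself.
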(event `DialogueForestOnLevelStart`
  (`/Game/VisualEffects/Font/2d_scenes/2d_scenes1/StoryAdvTemplate/Blueprints/Core/BP_StoryAdv_FunctionLibrary.DisablePlayerMovement`)
  (`self.EnableInput` (`GameplayStatics.GetPlayerController` 0))
  (`|ExecutionSequence`
    (:`then_0`
      (set `self.TextSetter` (`self.First Message`)))
    (:`then_1`
      (set `self.InsideBox` true)
      (bind _returnvalue (`|CreateWidget` "/Game/VisualEffects/Font/2d_scenes/Scenes/Forest/Text/text_forestLevelBP.text_forestLevelBP_C"))
      (bind _output_get (set `self.Text Forest 1` _returnvalue))
      (`UserWidget.AddToViewport` _output_get 0)
      (`/Game/VisualEffects/Font/2d_scenes/Scenes/Forest/Text/text_forestLevelBP.Initiate` (`self.Text Forest 1`))
      (`KismetSystemLibrary.Delay` (* (`KismetStringLibrary.Len` (`self.First Message`)) 0.03))
      (set `self.IsTextFinishedWriting?` true)
      (set `/Game/VisualEffects/Font/2d_scenes/Scenes/Forest/Text/text_forestLevelBP.Letter Text Delay` 0.03 (`self.Text Forest 1`)))))

(event `InputAction|Interact`
  (params (Key :type "Key Structure"))
  (bind _text_forest_1 (`self.Text Forest 1`))
  (bind _istextfinishedwriting_ (`self.IsTextFinishedWriting?`))
  (:`Pressed`
    (`KismetSystemLibrary.PrintString` "interact")
    (if (`self.InsideBox`)
      (bind _output_get (set `self.IntegerNumber` (+ (`self.IntegerNumber`) 1)))
      (switch `int` _output_get
        (:`1`
          (if _istextfinishedwriting_
            (set `self.IsTextFinishedWriting?` false)
            (`Widget.RemoveFromParent` (`self.Text Forest 1`))
            (`KismetSystemLibrary.Delay` (`self.Delay Time`))
            (set `self.TextSetter` (`self.Second Message`))
            (`GameplayStatics.CreateSound2D` (`self.Sound 2`) 1.0 1.0 0.0 null)
            (bind _returnvalue (`|CreateWidget` "/Game/VisualEffects/Font/2d_scenes/Scenes/Forest/Text/text_forestLevelBP.text_forestLevelBP_C"))
            (bind _output_get_2 (set `self.Text Forest 1` _returnvalue))
            (`UserWidget.AddToViewport` _output_get_2 0)
            (`/Game/VisualEffects/Font/2d_scenes/Scenes/Forest/Text/text_forestLevelBP.Initiate` (`self.Text Forest 1`))
            (`KismetSystemLibrary.PrintString` "Second Message")
            (set `/Game/VisualEffects/Font/2d_scenes/Scenes/Forest/Text/text_forestLevelBP.Letter Text Delay` 0.03 _text_forest_1)
            (`KismetSystemLibrary.Delay` (* (`KismetStringLibrary.Len` (`self.Second Message`)) 0.03))
            (set `self.IsTextFinishedWriting?` true)
            (else
              (set `/Game/VisualEffects/Font/2d_scenes/Scenes/Forest/Text/text_forestLevelBP.Letter Text Delay` 0.0 (`self.Text Forest 1`))
              (set `self.IntegerNumber` 0))))
        (:`2`
          (if _istextfinishedwriting_
            (set `self.IsTextFinishedWriting?` false)
            (`Widget.RemoveFromParent` (`self.Text Forest 1`))
            (`KismetSystemLibrary.Delay` (`self.Delay Time`))
            (set `self.TextSetter` (`self.Third Message`))
            (`GameplayStatics.CreateSound2D` (`self.Sound 3`) 1.0 1.0 0.0 null)
            (bind _returnvalue_2 (`|CreateWidget` "/Game/VisualEffects/Font/2d_scenes/Scenes/Forest/Text/text_forestLevelBP.text_forestLevelBP_C"))
            (bind _output_get_3 (set `self.Text Forest 1` _returnvalue_2))
            (`UserWidget.AddToViewport` _output_get_3 0)
            (`/Game/VisualEffects/Font/2d_scenes/Scenes/Forest/Text/text_forestLevelBP.Initiate` (`self.Text Forest 1`))
            (`KismetSystemLibrary.PrintString` "Third Message")
            (set `/Game/VisualEffects/Font/2d_scenes/Scenes/Forest/Text/text_forestLevelBP.Letter Text Delay` 0.03 _text_forest_1)
            (`KismetSystemLibrary.Delay` (* (`KismetStringLibrary.Len` (`self.Third Message`)) 0.03))
            (set `self.IsTextFinishedWriting?` true)
            (else
              (set `/Game/VisualEffects/Font/2d_scenes/Scenes/Forest/Text/text_forestLevelBP.Letter Text Delay` 0.0 (`self.Text Forest 1`))
              (set `self.IntegerNumber` 1))))
        (:`3`
          (if _istextfinishedwriting_
            (set `self.IsTextFinishedWriting?` false)
            (`KismetSystemLibrary.Delay` 0.1)
            (`self.DisableInput` (`GameplayStatics.GetPlayerController` 0))
            (set `self.InsideBox` false)
            (set `self.IntegerNumber` 0)
            (`/Game/VisualEffects/Font/2d_scenes/2d_scenes1/StoryAdvTemplate/Blueprints/Core/BP_StoryAdv_FunctionLibrary.EnablePlayerMovement`)
            (`self.FinishedTalking`)
            (`KismetSystemLibrary.Delay` 0.2)
            (`Widget.RemoveFromParent` (`self.Text Forest 1`))
            (set `/Game/VisualEffects/Font/2d_scenes/Scenes/Forest/Text/text_forestLevelBP.Letter Text Delay` 0.03 (`self.Text Forest 1`))
            (`self.K2_DestroyActor`)
            (else
              (set `/Game/VisualEffects/Font/2d_scenes/Scenes/Forest/Text/text_forestLevelBP.Letter Text Delay` 0.0 (`self.Text Forest 1`))
              (set `self.IntegerNumber` 2))))))))

(fn `UserConstructionScript`)

(fn `Write Text`
  (set `self.Built text` (`KismetTextLibrary.Conv_StringToText` (`KismetStringLibrary.Concat_StrStr` (`KismetTextLibrary.Conv_TextToString` (`self.Built text`)) (`KismetTextLibrary.Conv_TextToString` (`self.Current Character`))))))