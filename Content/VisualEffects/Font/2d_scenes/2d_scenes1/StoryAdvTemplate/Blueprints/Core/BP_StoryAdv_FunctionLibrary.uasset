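; Blueprint function library for the StoryAdv template that turns player movement off and on.
; DisablePlayerMovement makes the first player controller ignore move input, stops the pawn's movement component immediately and zeroes HeadTurnSpeed on the first VRPawn found in the level.
; EnablePlayerMovement restores move input and sets HeadTurnSpeed back to a hardcoded value rather than a saved one.
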(fn `DisablePlayerMovement`
  (`Controller.SetIgnoreMoveInput` (`GameplayStatics.GetPlayerController` null) true)
  (`MovementComponent.StopMovementImmediately` (`Pawn.GetMovementComponent` (`GameplayStatics.GetPlayerPawn` null)))
  (bind _outactors (`GameplayStatics.GetAllActorsOfClass` null "/Game/Player/VRPawn.VRPawn_C"))
  (set `/Game/Player/VRPawn.HeadTurnSpeed` 0.0 (`|GetArrayItem` _outactors)))

(fn `EnablePlayerMovement`
  (`Controller.SetIgnoreMoveInput` (`GameplayStatics.GetPlayerController` null) false)
  (bind _outactors (`GameplayStatics.GetAllActorsOfClass` null "/Game/Player/VRPawn.VRPawn_C"))
  (set `/Game/Player/VRPawn.HeadTurnSpeed` 2.5 (`|GetArrayItem` _outactors)))