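; Interaction zone actor that teleports the VR pawn to a target location through a fade transition, likely as a gate.
; Box overlap shows prompt text, registers the zone as the pawn's CurrentInteractZone and re-arms a DoOnce.
; Interact, when inside the box, plays the FadeIn sequence and camera fade, then teleports with a sound while movement is briefly disabled.
; FadeOut is unused, and a second sequence-playing chain is unconnected.
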(event `/Game/Blueprints/BPI_Interact.Interact`
  (`/Engine/EditorBlueprintResources/StandardMacros.DoOnce` false :!label _label
    (:`Completed`
      (`KismetSystemLibrary.PrintString` "GateInteraction")
      (if (`self.Is Inside box?`)
        (bind _outactors (`GameplayStatics.GetAllActorsOfClass` "/Script/LevelSequence.LevelSequenceActor"))
        (`LevelSequenceActor.SetSequence` _outactors (`self.FadeIn`))
        (`MovieSceneSequencePlayer.Play` (`LevelSequenceActor.SequencePlayer` (`|GetArrayItem` _outactors)))
        (`PlayerCameraManager.StartCameraFade` :`self` (`GameplayStatics.GetPlayerCameraManager` 0) :`ToAlpha` 1.0 :`Duration` 1.0 :`bShouldFadeAudio` true)
        (`/Game/VisualEffects/Font/2d_scenes/StoryAdvTemplate/Blueprints/Core/BP_StoryAdv_FunctionLibrary.DisablePlayerMovement`)
        (`KismetSystemLibrary.Delay` 1.0)
        (`GameplayStatics.PlaySound2D` (`self.Sound`) 1.0 1.0 0.0 null null)
        (bind _outactors_2 (`GameplayStatics.GetAllActorsOfClass` "/Game/Player/VRPawn.VRPawn_C"))
        (`self.K2_TeleportTo` (`|GetArrayItem` _outactors_2) (`self.K2_GetActorLocation` (`self.Location to Teleport to`)) (`self.Teleport Rotation`))
        (`KismetSystemLibrary.Delay` 1.0)
        (`/Game/VisualEffects/Font/2d_scenes/StoryAdvTemplate/Blueprints/Core/BP_StoryAdv_FunctionLibrary.EnablePlayerMovement`)))))

(event `self.Box.OnComponentBeginOverlap`
  (params (OverlappedComponent :type "PrimitiveComponent Object Reference") (OtherActor :type "Actor Object Reference") (OtherComp :type "PrimitiveComponent Object Reference") (OtherBodyIndex :type Integer) (bFromSweep :type Boolean) (SweepResult :type "HitResult Structure (by ref)"))
  (bind _asvrpawn (cast `/Game/Player/VRPawn` OtherActor))
  (set `/Game/Player/VRPawn.CurrentInteractZone` self _asvrpawn)
  (`SceneComponent.SetHiddenInGame` (`self.TextRender`) false true)
  (bind _output_get (set `self.Is Inside box?` true))
  (`KismetSystemLibrary.PrintString` (`KismetStringLibrary.Conv_BoolToString` _output_get))
  (goto _label :!via `Reset`))

(event `self.Box.OnComponentEndOverlap`
  (params (OverlappedComponent :type "PrimitiveComponent Object Reference") (OtherActor :type "Actor Object Reference") (OtherComp :type "PrimitiveComponent Object Reference") (OtherBodyIndex :type Integer))
  (bind _asvrpawn (cast `/Game/Player/VRPawn` OtherActor))
  (set `/Game/Player/VRPawn.CurrentInteractZone` null _asvrpawn)
  (`SceneComponent.SetHiddenInGame` (`self.TextRender`) true true)
  (bind _output_get (set `self.Is Inside box?` false))
  (`KismetSystemLibrary.PrintString` (`KismetStringLibrary.Conv_BoolToString` _output_get)))

(fn `UserConstructionScript`)