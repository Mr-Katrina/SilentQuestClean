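; Tree actor that billboards eight components (R through R7) toward the player camera, likely foliage cards.
; Every Tick, each component takes a look-at rotation to the camera manager's location and adds 90 degrees of pitch before setting its world rotation.
; The rotation passes through RInterpTo with no interp speed set, so it snaps to the target instead of easing.
; The construction script is empty.
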(event `self.ReceiveTick`
  (params (DeltaSeconds :type "Float (single-precision)"))
  (bind _r1 (`self.r1`))
  (bind _r3 (`self.r3`))
  (bind _r (`self.r`))
  (bind _r7 (`self.r7`))
  (bind _r6 (`self.r6`))
  (bind _r5 (`self.r5`))
  (bind _r4 (`self.r4`))
  (bind _r2 (`self.r2`))
  (bind (_returnvalue_roll _returnvalue_pitch _returnvalue_yaw) (`KismetMathLibrary.BreakRotator` (`KismetMathLibrary.RInterpTo` (`SceneComponent.K2_GetComponentRotation` _r6) (`KismetMathLibrary.FindLookAtRotation` (`SceneComponent.K2_GetComponentLocation` _r6) (`self.K2_GetActorLocation` (`GameplayStatics.GetPlayerCameraManager` 0))) DeltaSeconds)))
  (bind (_returnvalue_roll_2 _returnvalue_pitch_2 _returnvalue_yaw_2) (`KismetMathLibrary.BreakRotator` (`KismetMathLibrary.RInterpTo` (`SceneComponent.K2_GetComponentRotation` _r5) (`KismetMathLibrary.FindLookAtRotation` (`SceneComponent.K2_GetComponentLocation` _r5) (`self.K2_GetActorLocation` (`GameplayStatics.GetPlayerCameraManager` 0))) DeltaSeconds)))
  (bind (_returnvalue_roll_3 _returnvalue_pitch_3 _returnvalue_yaw_3) (`KismetMathLibrary.BreakRotator` (`KismetMathLibrary.RInterpTo` (`SceneComponent.K2_GetComponentRotation` _r4) (`KismetMathLibrary.FindLookAtRotation` (`SceneComponent.K2_GetComponentLocation` _r4) (`self.K2_GetActorLocation` (`GameplayStatics.GetPlayerCameraManager` 0))) DeltaSeconds)))
  (bind (_returnvalue_roll_4 _returnvalue_pitch_4 _returnvalue_yaw_4) (`KismetMathLibrary.BreakRotator` (`KismetMathLibrary.RInterpTo` (`SceneComponent.K2_GetComponentRotation` _r) (`KismetMathLibrary.FindLookAtRotation` (`SceneComponent.K2_GetComponentLocation` _r) (`self.K2_GetActorLocation` (`GameplayStatics.GetPlayerCameraManager` 0))) DeltaSeconds)))
  (bind (_returnvalue_roll_5 _returnvalue_pitch_5 _returnvalue_yaw_5) (`KismetMathLibrary.BreakRotator` (`KismetMathLibrary.RInterpTo` (`SceneComponent.K2_GetComponentRotation` _r1) (`KismetMathLibrary.FindLookAtRotation` (`SceneComponent.K2_GetComponentLocation` _r1) (`self.K2_GetActorLocation` (`GameplayStatics.GetPlayerCameraManager` 0))) DeltaSeconds)))
  (bind (_returnvalue_roll_6 _returnvalue_pitch_6 _returnvalue_yaw_6) (`KismetMathLibrary.BreakRotator` (`KismetMathLibrary.RInterpTo` (`SceneComponent.K2_GetComponentRotation` _r3) (`KismetMathLibrary.FindLookAtRotation` (`SceneComponent.K2_GetComponentLocation` _r3) (`self.K2_GetActorLocation` (`GameplayStatics.GetPlayerCameraManager` 0))) DeltaSeconds)))
  (bind (_returnvalue_roll_7 _returnvalue_pitch_7 _returnvalue_yaw_7) (`KismetMathLibrary.BreakRotator` (`KismetMathLibrary.RInterpTo` (`SceneComponent.K2_GetComponentRotation` _r2) (`KismetMathLibrary.FindLookAtRotation` (`SceneComponent.K2_GetComponentLocation` _r2) (`self.K2_GetActorLocation` (`GameplayStatics.GetPlayerCameraManager` 0))) DeltaSeconds)))
  (bind (_returnvalue_roll_8 _returnvalue_pitch_8 _returnvalue_yaw_8) (`KismetMathLibrary.BreakRotator` (`KismetMathLibrary.RInterpTo` (`SceneComponent.K2_GetComponentRotation` _r7) (`KismetMathLibrary.FindLookAtRotation` (`SceneComponent.K2_GetComponentLocation` _r7) (`self.K2_GetActorLocation` (`GameplayStatics.GetPlayerCameraManager` 0))) DeltaSeconds)))
  (`|ExecutionSequence`
    (:`then_0`
      (`SceneComponent.K2_SetWorldRotation` _r (`KismetMathLibrary.MakeRotator` _returnvalue_roll_4 (+ _returnvalue_pitch_4 90.0) _returnvalue_yaw_4) false false))
    (:`then_1`
      (`SceneComponent.K2_SetWorldRotation` _r1 (`KismetMathLibrary.MakeRotator` _returnvalue_roll_5 (+ _returnvalue_pitch_5 90.0) _returnvalue_yaw_5) false false))
    (:`then_2`
      (`SceneComponent.K2_SetWorldRotation` _r3 (`KismetMathLibrary.MakeRotator` _returnvalue_roll_6 (+ _returnvalue_pitch_6 90.0) _returnvalue_yaw_6) false false))
    (:`then_3`
      (`SceneComponent.K2_SetWorldRotation` _r7 (`KismetMathLibrary.MakeRotator` _returnvalue_roll_8 (+ _returnvalue_pitch_8 90.0) _returnvalue_yaw_8) false false))
    (:`then_4`
      (`SceneComponent.K2_SetWorldRotation` _r6 (`KismetMathLibrary.MakeRotator` _returnvalue_roll (+ _returnvalue_pitch 90.0) _returnvalue_yaw) false false))
    (:`then_5`
      (`SceneComponent.K2_SetWorldRotation` _r5 (`KismetMathLibrary.MakeRotator` _returnvalue_roll_2 (+ _returnvalue_pitch_2 90.0) _returnvalue_yaw_2) false false))
    (:`then_6`
      (`SceneComponent.K2_SetWorldRotation` _r4 (`KismetMathLibrary.MakeRotator` _returnvalue_roll_3 (+ _returnvalue_pitch_3 90.0) _returnvalue_yaw_3) false false))
    (:`then_7`
      (`SceneComponent.K2_SetWorldRotation` _r2 (`KismetMathLibrary.MakeRotator` _returnvalue_roll_7 (+ _returnvalue_pitch_7 90.0) _returnvalue_yaw_7) false false))))

(fn `UserConstructionScript`)