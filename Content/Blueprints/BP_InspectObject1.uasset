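; Inspectable VR object that shows a floating prompt and steps through subtitle lines on the VRPawn.
; Box overlap registers it as the pawn's CurrentInteractZone and toggles the prompt, which can rotate toward the camera.
; Each Interact advances SubtitleWhat; the first line locks movement and fades in the pawn's subtitle sphere and background through timeline-driven material parameters.
; Interacting past the last line fades them out, restores movement and resets.
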(event `self.ReceiveBeginPlay`
  ;[0 0 0] Set Floating Text
  (`TextRenderComponent.K2_SetText` (`self.InspectText`) (`self.Floating Text`))
  (`TextRenderComponent.K2_SetText` (`self.ShadowText`) (`self.Floating Text`)))

(event `EnhancedInput|/Game/VRTemplate/Input/Actions/IA_Interact`
  (params (ActionValue :type Boolean) (ElapsedSeconds :type "Float (double-precision)") (TriggeredSeconds :type "Float (double-precision)") (InputAction :type "InputAction Object Reference" :default "/Game/VRTemplate/Input/Actions/IA_Interact.IA_Interact")))

(event `/Game/Blueprints/BPI_Interact.Interact`
  (bind _subtitle_index (`self.Subtitle Index`))
  (bind _output (`|GetArrayItem` (`self.Subtitle What?`) _subtitle_index))
  ;[0 0 0] Conditions for Interacting
  (`KismetSystemLibrary.PrintString` "Interacted")
  (if (`self.Is Inside box?`)
    (if (< (`self.Subtitle Index`) (- (`KismetArrayLibrary.Array_Length` (`self.Subtitle What?`)) 1))
      ;[0 0 0] Switch on Int
      (`KismetSystemLibrary.PrintString` "Change Text")
      (`/Engine/EditorBlueprintResources/StandardMacros.IncrementInt` (`self.Subtitle Index`)
        (:`  `
          (`KismetSystemLibrary.PrintString` (`KismetTextLibrary.Conv_TextToString` _output))
          (`KismetSystemLibrary.PrintString` (`KismetStringLibrary.Conv_IntToString` _subtitle_index))
          (`SceneComponent.SetHiddenInGame` (`self.InspectText`) true true)
          (`|ExecutionSequence`
            (:`then_0`
              (bind _outactors (`GameplayStatics.GetAllActorsOfClass` "/Game/Player/VRPawn.VRPawn_C"))
              (bind _vr_subtitles (`/Game/Player/VRPawn.VR Subtitles` (`|GetArrayItem` _outactors)))
              (`TextRenderComponent.K2_SetText` _vr_subtitles _output)
              (`TextRenderComponent.K2_SetText` (`/Game/Player/VRPawn.VR Subtitles1` (`|GetArrayItem` _outactors)) _output)
              (`SceneComponent.SetHiddenInGame` _vr_subtitles false false)
              (`SceneComponent.SetHiddenInGame` (`/Game/Player/VRPawn.VR Subtitles1` (`|GetArrayItem` _outactors)) false false)
              (`SceneComponent.SetHiddenInGame` (`/Game/Player/VRPawn.TextBkg` (`|GetArrayItem` _outactors)) false false))
            (:`then_1`
              (if (== (`self.Subtitle Index`) 0)
                (`self.Dither`)
                (`/Game/VisualEffects/Font/2d_scenes/2d_scenes1/StoryAdvTemplate/Blueprints/Core/BP_StoryAdv_FunctionLibrary.DisablePlayerMovement`))))))
      (else
        (`KismetSystemLibrary.PrintString` "Finished Text")
        (`self.UnDither`)
        (bind _outactors_2 (`GameplayStatics.GetAllActorsOfClass` "/Game/Player/VRPawn.VRPawn_C"))
        (bind _output_2 (`|GetArrayItem` _outactors_2))
        (`SceneComponent.SetHiddenInGame` (`/Game/Player/VRPawn.VR Subtitles` _output_2) true false)
        (`SceneComponent.SetHiddenInGame` (`/Game/Player/VRPawn.VR Subtitles1` _output_2) true false)
        (`KismetSystemLibrary.Delay` 0.5)
        (`SceneComponent.SetHiddenInGame` (`/Game/Player/VRPawn.TextBkg` _output_2) true false)
        (`/Game/VisualEffects/Font/2d_scenes/StoryAdvTemplate/Blueprints/Core/BP_StoryAdv_FunctionLibrary.EnablePlayerMovement`)
        (`SceneComponent.SetHiddenInGame` (`self.InspectText`) false true)
        (set `self.Subtitle Index` -1)))))

(event `Dither`
  ;[0 0 0] Sphere Dither
  (bind _outactors (`GameplayStatics.GetAllActorsOfClass` "/Game/Player/VRPawn.VRPawn_C"))
  (`|ExecutionSequence`
    (:`then_0`
      (bind _output (`|GetArrayItem` _outactors))
      (bind _subtitle_sphere (`/Game/Player/VRPawn.Subtitle Sphere` _output))
      (bind _returnvalue (`PrimitiveComponent.CreateDynamicMaterialInstance` _subtitle_sphere 0 "/Game/Scenes/Subtitles/Text_Spher_Inst.Text_Spher_Inst" "None"))
      (bind _output_get (set `/Game/Player/VRPawn.Text Spere Dithering Material` _returnvalue _output))
      (`PrimitiveComponent.SetMaterial` _subtitle_sphere 0 _output_get)
      (bind (_direction _from_0_to_1) (`Timeline|Timeline_0` :!via `PlayFromStart`)
        (:`Update`
          (`MaterialInstanceDynamic.SetScalarParameterValue` _output_get "Percent" _from_0_to_1))))
    (:`then_1`
      (bind (_direction_2 _newtrack_0) (`Timeline|Timeline` :!via `PlayFromStart`)
        (:`Update`
          (`MeshComponent.SetScalarParameterValueOnMaterials` (`/Game/Player/VRPawn.TextBkg` _output) "Intensity" _newtrack_0))))))

(event `self.InteractionBox.OnComponentBeginOverlap`
  (params (OverlappedComponent :type "PrimitiveComponent Object Reference") (OtherActor :type "Actor Object Reference") (OtherComp :type "PrimitiveComponent Object Reference") (OtherBodyIndex :type Integer) (bFromSweep :type Boolean) (SweepResult :type "HitResult Structure (by ref)"))
  ;[0 0 0] Is Inside Trigger?
  (bind _asvrpawn (cast `/Game/Player/VRPawn` OtherActor))
  (set `/Game/Player/VRPawn.CurrentInteractZone` self _asvrpawn)
  (`SceneComponent.SetHiddenInGame` (`self.InspectText`) false true)
  (bind _output_get (set `self.Is Inside box?` true))
  (`KismetSystemLibrary.PrintString` (`KismetStringLibrary.Conv_BoolToString` _output_get)))

(event `self.InteractionBox.OnComponentEndOverlap`
  (params (OverlappedComponent :type "PrimitiveComponent Object Reference") (OtherActor :type "Actor Object Reference") (OtherComp :type "PrimitiveComponent Object Reference") (OtherBodyIndex :type Integer))
  ;[0 0 0] Is Inside Trigger?
  (bind _asvrpawn (cast `/Game/Player/VRPawn` OtherActor))
  (set `/Game/Player/VRPawn.CurrentInteractZone` null _asvrpawn)
  (`SceneComponent.SetHiddenInGame` (`self.InspectText`) true true)
  (bind _output_get (set `self.Is Inside box?` false))
  (`KismetSystemLibrary.PrintString` (`KismetStringLibrary.Conv_BoolToString` _output_get)))

(event `UnDither`
  ;[0 0 0] Sphere Dither
  (bind _outactors (`GameplayStatics.GetAllActorsOfClass` "/Game/Player/VRPawn.VRPawn_C"))
  (`|ExecutionSequence`
    (:`then_0`
      (bind _output (`|GetArrayItem` _outactors))
      (bind _subtitle_sphere (`/Game/Player/VRPawn.Subtitle Sphere` _output))
      (bind _returnvalue (`PrimitiveComponent.CreateDynamicMaterialInstance` _subtitle_sphere 0 "/Game/Scenes/Subtitles/Text_Spher_Inst.Text_Spher_Inst" "None"))
      (bind _output_get (set `/Game/Player/VRPawn.Text Spere Dithering Material` _returnvalue _output))
      (`PrimitiveComponent.SetMaterial` _subtitle_sphere 0 _output_get)
      (bind (_direction _from_0_to_1) (`Timeline|Timeline_1` :!via `PlayFromStart`)
        (:`Update`
          (`MaterialInstanceDynamic.SetScalarParameterValue` _output_get "Percent" _from_0_to_1))))
    (:`then_1`
      (bind (_direction_2 _newtrack_0) (`Timeline|Timeline_2` :!via `PlayFromStart`)
        (:`Update`
          (`MeshComponent.SetScalarParameterValueOnMaterials` (`/Game/Player/VRPawn.TextBkg` _output) "Intensity" _newtrack_0))))))

(event `self.ReceiveTick`
  (params (DeltaSeconds :type "Float (single-precision)"))
  ;[0 0 0] Rotate "Inspect?" Text Towards Player
  (if (`self.RotatableText?`)
    (`SceneComponent.K2_SetWorldRotation` (`self.InspectText`) (`KismetMathLibrary.RInterpTo` (`SceneComponent.K2_GetComponentRotation` (`self.InspectText`)) (`KismetMathLibrary.FindLookAtRotation` (`SceneComponent.K2_GetComponentLocation` (`self.InspectText`)) (`self.K2_GetActorLocation` (`GameplayStatics.GetPlayerCameraManager` 0))) DeltaSeconds 2.0) false false)))

(fn `UserConstructionScript`)