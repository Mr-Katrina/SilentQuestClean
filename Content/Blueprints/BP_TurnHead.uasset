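; Trigger actor that turns the VR pawn to face a TargetLocation actor, either on overlap or through the StartRotation event.
; Each path runs its own timeline, lerping the pawn's rotation toward a look-at rotation at the pawn's own height, keeping it level.
; StartRotation uses a stored pawn reference instead of the overlapping actor.
; A shared flag blocks re-triggering until a delay started from the timeline update clears it.
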(event `self.ReceiveActorBeginOverlap`
  (params (OtherActor :type "Actor Object Reference"))
  (bind (_returnvalue_x _returnvalue_y) (`KismetMathLibrary.BreakVector` (`self.K2_GetActorLocation` (`self.TargetLocation`))))
  (if (not (`self.Is AlreadyRotating?`))
    (set `self.Is AlreadyRotating?` true)
    (bind _asvrpawn (cast `/Game/Player/VRPawn` OtherActor))
    (bind (_direction _newtrack_0) (`Timeline|lerp` :!via `PlayFromStart`)
      (:`Update`
        (`KismetSystemLibrary.PrintString` "Is Lerping")
        (bind (_returnvalue_x_2 _returnvalue_y_2 _returnvalue_z) (`KismetMathLibrary.BreakVector` (`self.K2_GetActorLocation` _asvrpawn)))
        (`self.K2_SetActorRotation` _asvrpawn (`KismetMathLibrary.RLerp` (`self.K2_GetActorRotation` _asvrpawn) (`KismetMathLibrary.FindLookAtRotation` (`KismetMathLibrary.MakeVector` _returnvalue_x_2 _returnvalue_y_2 _returnvalue_z) (`KismetMathLibrary.MakeVector` _returnvalue_x _returnvalue_y _returnvalue_z)) _newtrack_0 true) false)
        (`KismetSystemLibrary.Delay` 0.98)
        (set `self.Is AlreadyRotating?` false)))))

(event `Start Rotation`
  (bind (_returnvalue_x _returnvalue_y) (`KismetMathLibrary.BreakVector` (`self.K2_GetActorLocation` (`self.TargetLocation`))))
  (bind (_returnvalue_x_2 _returnvalue_y_2 _returnvalue_z) (`KismetMathLibrary.BreakVector` (`self.K2_GetActorLocation` (`self.AsVrPawnInput`))))
  (if (not (`self.Is AlreadyRotating?`))
    (set `self.Is AlreadyRotating?` true)
    (bind (_direction _newtrack_0) (`Timeline|Timeline` :!via `PlayFromStart`)
      (:`Update`
        (`KismetSystemLibrary.PrintString` "Is Lerping")
        (`self.K2_SetActorRotation` (`self.AsVrPawnInput`) (`KismetMathLibrary.RLerp` (`self.K2_GetActorRotation` (`self.AsVrPawnInput`)) (`KismetMathLibrary.FindLookAtRotation` (`KismetMathLibrary.MakeVector` _returnvalue_x_2 _returnvalue_y_2 _returnvalue_z) (`KismetMathLibrary.MakeVector` _returnvalue_x _returnvalue_y _returnvalue_z)) _newtrack_0 true) false)
        (`KismetSystemLibrary.Delay` 0.98)
        (set `self.Is AlreadyRotating?` false)))))

(fn `UserConstructionScript`)