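; VR subtitle actor that shows a sequence of text lines on the VRPawn's subtitle components.
; Once started, StartSubtitle or each completed IA_Interact press advances through the SubtitleWhat array.
; The first line disables player movement and uses timelines to dither the pawn's subtitle sphere and drive the text background intensity.
; After the last line it reverses the effect, hides the text, triggers the follow-up action, restores movement and destroys itself.
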(event `EnhancedInput|/Game/VRTemplate/Input/Actions/IA_Interact`
  (params (ActionValue :type Boolean) (ElapsedSeconds :type "Float (double-precision)") (TriggeredSeconds :type "Float (double-precision)") (InputAction :type "InputAction Object Reference" :default "/Game/VRTemplate/Input/Actions/IA_Interact.IA_Interact"))
  (bind _output (`|GetArrayItem` (`self.Subtitle What?`) (`self.Subtitle Index`)))
  ;[0 0 0] Conditions for Interacting
  (:`Completed`
    (if (`self.StartedSubtitle?`) :!label _label
      (if (< (`self.Subtitle Index`) (- (`KismetArrayLibrary.Array_Length` (`self.Subtitle What?`)) 1))
        ;[0 0 0] Switch on Int
        (`KismetSystemLibrary.PrintString` "Change Text")
        (`/Engine/EditorBlueprintResources/StandardMacros.IncrementInt` (`self.Subtitle Index`)
          (:`  `
            (`KismetSystemLibrary.PrintString` (`KismetTextLibrary.Conv_TextToString` _output))
            (`|ExecutionSequence`
              (:`then_0`
                (bind _outactors (`GameplayStatics.GetAllActorsOfClass` "/Game/Player/VRPawn.VRPawn_C"))
                (bind _vr_subtitles (`/Game/Player/VRPawn.VR Subtitles` (`|GetArrayItem` _outactors)))
                (`TextRenderComponent.K2_SetText` _vr_subtitles _output)
                (`TextRenderComponent.K2_SetText` (`/Game/Player/VRPawn.VR Subtitles1` (`|GetArrayItem` _outactors)) _output)
                (`SceneComponent.SetHiddenInGame` _vr_subtitles false false)
                (`SceneComponent.SetHiddenInGame` (`/Game/Player/VRPawn.VR Subtitles1` (`|GetArrayItem` _outactors)) false false)
                (`SceneComponent.SetHiddenInGame` (`/Game/Player/VRPawn.TextBkg` (`|GetArrayItem` _outactors)) false false))
              (:`then_1`
                (if (== (`self.Subtitle Index`) 0)
                  (`self.Dither`)
                  (`/Game/VisualEffects/Font/2d_scenes/StoryAdvTemplate/Blueprints/Core/BP_StoryAdv_FunctionLibrary.DisablePlayerMovement`))))))
        (else
          (`KismetSystemLibrary.PrintString` "Finished Text")
          (`self.UnDither`)
          (bind _outactors_2 (`GameplayStatics.GetAllActorsOfClass` "/Game/Player/VRPawn.VRPawn_C"))
          (bind _output_2 (`|GetArrayItem` _outactors_2))
          (`SceneComponent.SetHiddenInGame` (`/Game/Player/VRPawn.VR Subtitles` _output_2) true false)
          (`SceneComponent.SetHiddenInGame` (`/Game/Player/VRPawn.VR Subtitles1` _output_2) true false)
          (`KismetSystemLibrary.Delay` 0.5)
          (`SceneComponent.SetHiddenInGame` (`/Game/Player/VRPawn.TextBkg` _output_2) true false)
          (`self.Do Action After Text`)
          (`/Game/VisualEffects/Font/2d_scenes/StoryAdvTemplate/Blueprints/Core/BP_StoryAdv_FunctionLibrary.EnablePlayerMovement`)
          (`self.K2_DestroyActor`))))))

(event `Start Subtitle`
  ;[0 0 0] Conditions for Interacting
  (goto _label))

(event `Dither`
  ;[0 0 0] Sphere Dither
  (bind _outactors (`GameplayStatics.GetAllActorsOfClass` "/Game/Player/VRPawn.VRPawn_C"))
  (`|ExecutionSequence`
    (:`then_0`
      (bind _output (`|GetArrayItem` _outactors))
      (bind _subtitle_sphere (`/Game/Player/VRPawn.Subtitle Sphere` _output))
      (bind _returnvalue (`PrimitiveComponent.CreateDynamicMaterialInstance` _subtitle_sphere 0 "/Game/Scenes/Subtitles/Text_Spher_Inst.Text_Spher_Inst" "None"))
      (bind _output_get (set `/Game/Player/VRPawn.Text Spere Dithering Material` _returnvalue _output))
      (`PrimitiveComponent.SetMaterial` _subtitle_sphere 0 _output_get)
      (bind (_direction _from_0_to_1) (`Timeline|Timeline_0` :!via `PlayFromStart`)
        (:`Update`
          (`MaterialInstanceDynamic.SetScalarParameterValue` _output_get "Percent" _from_0_to_1))))
    (:`then_1`
      (bind (_direction_2 _newtrack_0) (`Timeline|Timeline` :!via `PlayFromStart`)
        (:`Update`
          (`MeshComponent.SetScalarParameterValueOnMaterials` (`/Game/Player/VRPawn.TextBkg` _output) "Intensity" _newtrack_0))))))

(event `UnDither`
  ;[0 0 0] Sphere Dither
  (bind _outactors (`GameplayStatics.GetAllActorsOfClass` "/Game/Player/VRPawn.VRPawn_C"))
  (`|ExecutionSequence`
    (:`then_0`
      (bind _output (`|GetArrayItem` _outactors))
      (bind _subtitle_sphere (`/Game/Player/VRPawn.Subtitle Sphere` _output))
      (bind _returnvalue (`PrimitiveComponent.CreateDynamicMaterialInstance` _subtitle_sphere 0 "/Game/Scenes/Subtitles/Text_Spher_Inst.Text_Spher_Inst" "None"))
      (bind _output_get (set `/Game/Player/VRPawn.Text Spere Dithering Material` _returnvalue _output))
      (`PrimitiveComponent.SetMaterial` _subtitle_sphere 0 _output_get)
      (bind (_direction _from_0_to_1) (`Timeline|Timeline_1` :!via `PlayFromStart`)
        (:`Update`
          (`MaterialInstanceDynamic.SetScalarParameterValue` _output_get "Percent" _from_0_to_1))))
    (:`then_1`
      (bind (_direction_2 _newtrack_0) (`Timeline|Timeline_2` :!via `PlayFromStart`)
        (:`Update`
          (`MeshComponent.SetScalarParameterValueOnMaterials` (`/Game/Player/VRPawn.TextBkg` _output) "Intensity" _newtrack_0))))))

(fn `UserConstructionScript`)