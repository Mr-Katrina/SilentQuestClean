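; BP_PlayMovie is a one-shot VR movie trigger, started on BeginPlay, box overlap or the PlayMovie event.
; It disables movement, possesses a spectator pawn, resets headset orientation, hides fog and post-process, then hands media to BP_Movie for playback.
; After a duration Delay, or when EnablePP is called, it restores the effects and VRPawn control, then destroys itself.
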(event `PlayMovie`
  ;[0 0 0] Condition
  ;[0 0 0] Change To Spectator
  (`/Game/VisualEffects/Font/2d_scenes/StoryAdvTemplate/Blueprints/Core/BP_StoryAdv_FunctionLibrary.DisablePlayerMovement` :!label _label)
  (`Controller.Possess` (`GameplayStatics.GetPlayerController` 0) (`self.VRSpectator`))
  (`HeadMountedDisplayFunctionLibrary.ResetOrientationAndPosition` 0.0)
  ;[0 0 0] Disable PP
  (`SceneComponent.SetVisibility` (`Actor.RootComponent` (`self.Fog To Disable`)) false false)
  (set `PostProcessVolume.bEnabled` false (`self.PostProcess To Disable`))
  ;[0 0 0] Play Video
  (bind _outactors (`GameplayStatics.GetAllActorsOfClass` "/Game/Blueprints/Movie/BP_Movie.BP_Movie_C"))
  (bind _output (`|GetArrayItem` _outactors))
  (set `/Game/Blueprints/Movie/BP_Movie.Media` (`self.Media`) _output)
  (set `/Game/Blueprints/Movie/BP_Movie.MediaSource` (`self.Media Source`) _output)
  (set `/Game/Blueprints/Movie/BP_Movie.MovieMaterial` (`self.Movie Material`) _output)
  (`/Game/Blueprints/Movie/BP_Movie.PlayVideo` _outactors)
  (`KismetSystemLibrary.Delay` (`self.Movie Duration`))
  ;[0 0 0] Enable PP
  (`SceneComponent.SetVisibility` (`Actor.RootComponent` (`self.Fog To Disable`)) true false :!label _label_2)
  (set `PostProcessVolume.bEnabled` true (`self.PostProcess To Disable`))
  ;[0 0 0] Change Back To Player
  (bind _outactors_2 (`GameplayStatics.GetAllActorsOfClass` "/Game/Player/VRPawn.VRPawn_C"))
  (`Controller.Possess` (`GameplayStatics.GetPlayerController` 0) (`|GetArrayItem` _outactors_2))
  (`HeadMountedDisplayFunctionLibrary.ResetOrientationAndPosition` 0.0)
  (`/Game/VisualEffects/Font/2d_scenes/2d_scenes1/StoryAdvTemplate/Blueprints/Core/BP_StoryAdv_FunctionLibrary.EnablePlayerMovement`)
  (`KismetSystemLibrary.Delay` 0.2)
  (`self.K2_DestroyActor`))

(event `self.ReceiveBeginPlay`
  ;[0 0 0] Condition
  (if (`self.PlayOnStart?`)
    (goto _label)))

(event `EnablePP`
  (goto _label_2))

(event `self.Box.OnComponentBeginOverlap`
  (params (OverlappedComponent :type "PrimitiveComponent Object Reference") (OtherActor :type "Actor Object Reference") (OtherComp :type "PrimitiveComponent Object Reference") (OtherBodyIndex :type Integer) (bFromSweep :type Boolean) (SweepResult :type "HitResult Structure (by ref)"))
  ;[0 0 0] Condition
  (if (`self.PlayOnOverlap?`)
    (goto _label)))

(fn `UserConstructionScript`)