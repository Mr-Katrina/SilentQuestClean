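; Blueprint that shows timed subtitles on the VR pawn, with events to fade a dithered backdrop.
; StartSubtitle increments an index into a text array, fills both pawn text components, hides them and their background after delays, then resets the index.
; Separate Dither and UnDither events use timelines to drive a dynamic sphere material's Percent and the background's Intensity.
; Every event finds the pawn as the first VRPawn actor.
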(event `Start Subtitle`
  (bind _output (`|GetArrayItem` (`self.TSubtitle What?`) (`self.TSubtitle Index`)))
  ;[0 0 0] Subtitle
  (`KismetSystemLibrary.PrintString` "Change Text")
  (`/Engine/EditorBlueprintResources/StandardMacros.IncrementInt` (`self.TSubtitle Index`)
    (:`  `
      (`KismetSystemLibrary.PrintString` (`KismetTextLibrary.Conv_TextToString` _output))
      (bind _outactors (`GameplayStatics.GetAllActorsOfClass` "/Game/Player/VRPawn.VRPawn_C"))
      (bind _vr_subtitles (`/Game/Player/VRPawn.VR Subtitles` (`|GetArrayItem` _outactors)))
      (`TextRenderComponent.K2_SetText` _vr_subtitles _output)
      (`TextRenderComponent.K2_SetText` (`/Game/Player/VRPawn.VR Subtitles1` (`|GetArrayItem` _outactors)) _output)
      (`SceneComponent.SetHiddenInGame` _vr_subtitles false false)
      (`SceneComponent.SetHiddenInGame` (`/Game/Player/VRPawn.VR Subtitles1` (`|GetArrayItem` _outactors)) false false)
      (`SceneComponent.SetHiddenInGame` (`/Game/Player/VRPawn.TextBkg` (`|GetArrayItem` _outactors)) false false)
      (`KismetSystemLibrary.Delay` (`self.Duration`))
      (bind _outactors_2 (`GameplayStatics.GetAllActorsOfClass` "/Game/Player/VRPawn.VRPawn_C"))
      (bind _output_2 (`|GetArrayItem` _outactors_2))
      (`SceneComponent.SetHiddenInGame` (`/Game/Player/VRPawn.VR Subtitles` _output_2) true false)
      (`SceneComponent.SetHiddenInGame` (`/Game/Player/VRPawn.VR Subtitles1` _output_2) true false)
      (`KismetSystemLibrary.Delay` 0.5)
      (`SceneComponent.SetHiddenInGame` (`/Game/Player/VRPawn.TextBkg` _output_2) true false)
      (set `self.TSubtitle Index` -1))))

(event `Dither`
  ;[0 0 0] Sphere Dither
  (bind _outactors (`GameplayStatics.GetAllActorsOfClass` "/Game/Player/VRPawn.VRPawn_C"))
  (`|ExecutionSequence`
    (:`then_0`
      (bind _output (`|GetArrayItem` _outactors))
      (bind _subtitle_sphere (`/Game/Player/VRPawn.Subtitle Sphere` _output))
      (bind _returnvalue (`PrimitiveComponent.CreateDynamicMaterialInstance` _subtitle_sphere 0 "/Game/Scenes/Subtitles/Text_Spher_Inst.Text_Spher_Inst" "None"))
      (bind _output_get (set `/Game/Player/VRPawn.Text Spere Dithering Material` _returnvalue _output))
      (`PrimitiveComponent.SetMaterial` _subtitle_sphere 0 _output_get)
      (bind (_direction _from_0_to_1) (`Timeline|Timeline_0` :!via `PlayFromStart`)
        (:`Update`
          (`MaterialInstanceDynamic.SetScalarParameterValue` _output_get "Percent" _from_0_to_1))))
    (:`then_1`
      (bind (_direction_2 _newtrack_0) (`Timeline|Timeline` :!via `PlayFromStart`)
        (:`Update`
          (`MeshComponent.SetScalarParameterValueOnMaterials` (`/Game/Player/VRPawn.TextBkg` _output) "Intensity" _newtrack_0))))))

(event `UnDither`
  ;[0 0 0] Sphere Dither
  (bind _outactors (`GameplayStatics.GetAllActorsOfClass` "/Game/Player/VRPawn.VRPawn_C"))
  (`|ExecutionSequence`
    (:`then_0`
      (bind _output (`|GetArrayItem` _outactors))
      (bind _subtitle_sphere (`/Game/Player/VRPawn.Subtitle Sphere` _output))
      (bind _returnvalue (`PrimitiveComponent.CreateDynamicMaterialInstance` _subtitle_sphere 0 "/Game/Scenes/Subtitles/Text_Spher_Inst.Text_Spher_Inst" "None"))
      (bind _output_get (set `/Game/Player/VRPawn.Text Spere Dithering Material` _returnvalue _output))
      (`PrimitiveComponent.SetMaterial` _subtitle_sphere 0 _output_get)
      (bind (_direction _from_0_to_1) (`Timeline|Timeline_1` :!via `PlayFromStart`)
        (:`Update`
          (`MaterialInstanceDynamic.SetScalarParameterValue` _output_get "Percent" _from_0_to_1))))
    (:`then_1`
      (bind (_direction_2 _newtrack_0) (`Timeline|Timeline_2` :!via `PlayFromStart`)
        (:`Update`
          (`MeshComponent.SetScalarParameterValueOnMaterials` (`/Game/Player/VRPawn.TextBkg` _output) "Intensity" _newtrack_0))))))

(fn `UserConstructionScript`)