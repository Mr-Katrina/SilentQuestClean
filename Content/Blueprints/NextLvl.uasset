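; NextLvl is a level-exit trigger that loads another level when the player interacts inside its box.
; Box overlap events show or hide a text prompt and set the IsInsideBox flag that gates the IA_Interact input.
; A one-shot interaction plays a sound, disables player movement, assigns FadeOut to every LevelSequenceActor found and plays the first.
; After a short delay for the fade, it opens the referenced Level.
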(event `EnhancedInput|/Game/VRTemplate/Input/Actions/IA_Interact`
  (params (ActionValue :type Boolean) (ElapsedSeconds :type "Float (double-precision)") (TriggeredSeconds :type "Float (double-precision)") (InputAction :type "InputAction Object Reference" :default "/Game/VRTemplate/Input/Actions/IA_Interact.IA_Interact"))
  (:`Triggered`
    (if (`self.Is Inside box?`)
      (`/Engine/EditorBlueprintResources/StandardMacros.DoOnce` false
        (:`Completed`
          (`GameplayStatics.PlaySound2D` (`self.Sound`) 1.0 1.0 0.0 null null)
          (`/Game/VisualEffects/Font/2d_scenes/StoryAdvTemplate/Blueprints/Core/BP_StoryAdv_FunctionLibrary.DisablePlayerMovement`)
          (bind _outactors (`GameplayStatics.GetAllActorsOfClass` "/Script/LevelSequence.LevelSequenceActor"))
          (`LevelSequenceActor.SetSequence` _outactors (`self.FadeOut`))
          (`MovieSceneSequencePlayer.Play` (`LevelSequenceActor.SequencePlayer` (`|GetArrayItem` _outactors)))
          (`KismetSystemLibrary.Delay` 2.0)
          (`GameplayStatics.OpenLevelBySoftObjectPtr` (`self.Level`)))))))

(event `self.Box.OnComponentBeginOverlap`
  (params (OverlappedComponent :type "PrimitiveComponent Object Reference") (OtherActor :type "Actor Object Reference") (OtherComp :type "PrimitiveComponent Object Reference") (OtherBodyIndex :type Integer) (bFromSweep :type Boolean) (SweepResult :type "HitResult Structure (by ref)"))
  (`SceneComponent.SetHiddenInGame` (`self.TextRender`) false true)
  (bind _output_get (set `self.Is Inside box?` true))
  (`KismetSystemLibrary.PrintString` (`KismetStringLibrary.Conv_BoolToString` _output_get)))

(event `self.Box.OnComponentEndOverlap`
  (params (OverlappedComponent :type "PrimitiveComponent Object Reference") (OtherActor :type "Actor Object Reference") (OtherComp :type "PrimitiveComponent Object Reference") (OtherBodyIndex :type Integer))
  (`SceneComponent.SetHiddenInGame` (`self.TextRender`) true true)
  (bind _output_get (set `self.Is Inside box?` false))
  (`KismetSystemLibrary.PrintString` (`KismetStringLibrary.Conv_BoolToString` _output_get)))

(fn `UserConstructionScript`)