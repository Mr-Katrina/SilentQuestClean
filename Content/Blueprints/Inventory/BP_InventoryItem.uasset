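; BP_InventoryItem is a grabbable VR inventory item that shows its inspect text as pawn subtitles while held.
; Grabbing reveals the text and disables player movement; dropping hides it, re-enables movement and resets the subtitle index.
; An unfinished return-to-place routine uses a timeline to move the item home with physics toggled, but its original-transform capture and drop binding are disconnected and never run.
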(event `self.ReceiveBeginPlay`
  ;[0 0 0] Trying to make it so that after you drop it, it goes back in it's place
)

(event `OnDropped_Event`
  (params (SelfReference :type "/Game/Blueprints/Environment/RandomPickables/GrabComponent Object Reference"))
  ;[0 0 0] Trying to make it so that after you drop it, it goes back in it's place
  (`KismetSystemLibrary.Delay` 0.2)
  (`PrimitiveComponent.SetSimulatePhysics` (`self.StaticMesh`) false)
  (bind (_direction _alpha) (`Timeline|ReturnTimeline`)
    (:`Update`
      (`self.K2_SetActorLocation` (`KismetMathLibrary.VLerp` (`self.K2_GetActorLocation`) (`self.Original Location`) _alpha) true)
      (`self.K2_SetActorRotation` (`KismetMathLibrary.RInterpTo` (`self.K2_GetActorRotation`) (`self.Original Rotation`) 0.016 1.0))
      (`KismetSystemLibrary.Delay` 1.0)
      (`PrimitiveComponent.SetSimulatePhysics` (`self.StaticMesh`) true))))

(event `self.GrabComponent.OnGrabbed`
  (params (MotionController :type "MotionControllerComponent Object Reference") (SelfReference :type "/Game/Blueprints/Environment/RandomPickables/GrabComponent Object Reference"))
  (bind _inventory_inspect_text (`self.Inventory Inspect Text`))
  ;[0 0 0] Conditions for Interacting
  (`KismetSystemLibrary.PrintString` "Interacted")
  ;[0 0 0] Switch on Int
  (`KismetSystemLibrary.PrintString` (`KismetTextLibrary.Conv_TextToString` _inventory_inspect_text))
  (`|ExecutionSequence`
    (:`then_0`
      (bind _outactors (`GameplayStatics.GetAllActorsOfClass` "/Game/Player/VRPawn.VRPawn_C"))
      (bind _vr_subtitles (`/Game/Player/VRPawn.VR Subtitles` (`|GetArrayItem` _outactors)))
      (`TextRenderComponent.K2_SetText` _vr_subtitles _inventory_inspect_text)
      (`TextRenderComponent.K2_SetText` (`/Game/Player/VRPawn.VR Subtitles1` (`|GetArrayItem` _outactors)) _inventory_inspect_text)
      (`SceneComponent.SetHiddenInGame` _vr_subtitles false false)
      (`SceneComponent.SetHiddenInGame` (`/Game/Player/VRPawn.VR Subtitles1` (`|GetArrayItem` _outactors)) false false)
      (`SceneComponent.SetHiddenInGame` (`/Game/Player/VRPawn.TextBkg` (`|GetArrayItem` _outactors)) false false))
    (:`then_1`
      (`/Game/VisualEffects/Font/2d_scenes/2d_scenes1/StoryAdvTemplate/Blueprints/Core/BP_StoryAdv_FunctionLibrary.DisablePlayerMovement`))))

(event `self.GrabComponent.OnDropped`
  (params (SelfReference :type "/Game/Blueprints/Environment/RandomPickables/GrabComponent Object Reference"))
  ;[0 0 0] Conditions for Interacting
  ;[0 0 0] Switch on Int
  (`KismetSystemLibrary.PrintString` "Finished Text")
  (bind _outactors (`GameplayStatics.GetAllActorsOfClass` "/Game/Player/VRPawn.VRPawn_C"))
  (bind _output (`|GetArrayItem` _outactors))
  (`SceneComponent.SetHiddenInGame` (`/Game/Player/VRPawn.VR Subtitles` _output) true false)
  (`SceneComponent.SetHiddenInGame` (`/Game/Player/VRPawn.VR Subtitles1` _output) true false)
  (`KismetSystemLibrary.Delay` 0.5)
  (`SceneComponent.SetHiddenInGame` (`/Game/Player/VRPawn.TextBkg` _output) true false)
  (`/Game/VisualEffects/Font/2d_scenes/StoryAdvTemplate/Blueprints/Core/BP_StoryAdv_FunctionLibrary.EnablePlayerMovement`)
  (set `self.Subtitle Index` -1))

(fn `UserConstructionScript`)